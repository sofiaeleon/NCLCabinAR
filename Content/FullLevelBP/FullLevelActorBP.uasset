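; FullLevelActorBP is a level actor with a roof that can be raised and lowered.
; ToggleRoof shifts a static mesh component vertically by a fixed local offset, down when the roof is up and up otherwise, then flips the RoofIsUp flag.
; The move is instant and unswept, and the event graph and construction script are empty, so ToggleRoof is the only logic in the graphs.
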(event EventBeginPlay)

(event Collision|EventActorBeginOverlap
  (params (OtherActor :type Actor%20Object%20Reference)))

(event EventTick
  (params (DeltaSeconds :type Float%20%28single-precision%29)))

(fn ConstructionScript)

(fn ToggleRoof
  (if (Variables|Default|GetRoofIsUp)
    (Variables|Default|SetTranslateValue -5e+02)
    (else
      (Variables|Default|SetTranslateValue 5e+02)))
  (Class|SceneComponent|AddLocalTransform (Variables|Default|GetStaticMeshComponent0127) (Math|Transform|MakeTransform (Math|Vector|MakeVector 0.0 0.0 (Variables|Default|GetTranslateValue))) false false)
  (Variables|Default|SetRoofIsUp (not (Variables|Default|GetRoofIsUp))))